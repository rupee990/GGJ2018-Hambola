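; Two-ended pipe actor that sends Tagged and Untagged characters along a spline from either end.
; Every Tick polls both end volumes, handling the first overlapping Tagged character and all Untagged ones.
; It calls each character's Pipe function with the spline, a direction sign per end and a force along that end's arrow, leaving movement to the character.
; Overlap events are empty, and older teleport-and-launch logic remains disconnected.
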(event EventTick
  (params (DeltaSeconds :type Float%20%28single-precision%29))
  (bind _self self)
  (bind _pipeend (Variables|Default|GetPipeEnd))
  (bind _spline (Variables|Default|GetSpline))
  (bind _force (Variables|Default|GetForce))
  (bind _force_2 (Variables|Default|GetForce))
  (bind _spline_2 (Variables|Default|GetSpline))
  (bind _pipestart (Variables|Default|GetPipeStart))
  (bind _arrow1 (Variables|Default|GetArrow1))
  (bind _arrow (Variables|Default|GetArrow))
  (bind _returnvalue (Math|Vector|GetForwardVector _arrow1))
  (bind _returnvalue_2 (Math|Vector|GetForwardVector _arrow))
  (bind _returnvalue_3 (* _returnvalue _force))
  (bind _returnvalue_4 (* _returnvalue_2 _force_2))
  (Utilities|FlowControl|Sequence
    (:then_0
      (bind _astagged (Utilities|Casting|CastToTagged (Utilities|Array|Get(acopy) (Collision|GetOverlappingActors _pipeend "/Game/Blueprints/Tagged/Tagged.Tagged_C" :!class /Script/Engine.PrimitiveComponent))))
      (Default|Pipe _astagged _spline -1.0 _returnvalue_4 self))
    (:then_1
      (for _array_element (Collision|GetOverlappingActors _pipeend "/Game/Blueprints/untagged/untagged.untagged_C" :!class /Script/Engine.PrimitiveComponent)
        (bind _asuntagged (Utilities|Casting|CastTountagged _array_element))
        (Default|Pipe _asuntagged _spline -1.0 _returnvalue_4 self)))
    (:then_2
      (bind _astagged_2 (Utilities|Casting|CastToTagged (Utilities|Array|Get(acopy) (Collision|GetOverlappingActors _pipestart "/Game/Blueprints/Tagged/Tagged.Tagged_C" :!class /Script/Engine.PrimitiveComponent))))
      (Default|Pipe _astagged_2 _spline_2 1.0 _returnvalue_3 _self))
    (:then_3
      (for _array_element_2 (Collision|GetOverlappingActors _pipestart "/Game/Blueprints/untagged/untagged.untagged_C" :!class /Script/Engine.PrimitiveComponent)
        (bind _asuntagged_2 (Utilities|Casting|CastTountagged _array_element_2))
        (Default|Pipe _asuntagged_2 _spline_2 1.0 _returnvalue_3 _self)))))

(event Collision|EventActorBeginOverlap
  (params (OtherActor :type Actor%20Object%20Reference)))

(event Collision|EventActorEndOverlap
  (params (OtherActor :type Actor%20Object%20Reference)))

(fn ConstructionScript)