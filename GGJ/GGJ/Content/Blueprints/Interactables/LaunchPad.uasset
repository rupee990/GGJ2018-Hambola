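; Launch pad interactable that flings overlapping player characters along a fixed direction.
; On actor overlap it accepts actors whose first tag is "untagged" or "Tagged" and casts them to the Tagged character class.
; It snaps the character to CollisionFront's location and rotation, keeping its scale, then launches it along that component's up vector times Force, overriding existing velocity.
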(event Collision|EventActorBeginOverlap
  (params (OtherActor :type Actor%20Object%20Reference))
  (bind _tags (Variables|/Script/Engine.Actor|GetTags OtherActor))
  (bind _collisionfront (Variables|Default|GetCollisionFront))
  (bind _output (Utilities|Array|Get(acopy) _tags))
  (if (or (Utilities|Name|Equal(Name) _output "untagged") (Utilities|Name|Equal(Name) _output "Tagged"))
    (bind _astagged (Utilities|Casting|CastToTagged OtherActor))
    (Transformation|SetWorldTransform (Variables|/Script/Engine.Actor|GetRootComponent _astagged) (Math|Transform|MakeTransform (Transformation|GetWorldLocation _collisionfront) (Transformation|GetWorldRotation _collisionfront) (Transformation|GetActorScale3D OtherActor)) false false)
    (Character|LaunchCharacter _astagged (* (Math|Vector|GetUpVector _collisionfront) (Variables|Default|GetForce)) true true)))

(fn ConstructionScript)