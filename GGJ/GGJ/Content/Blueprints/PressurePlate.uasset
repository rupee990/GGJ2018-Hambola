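; Pressure plate actor that triggers a linked trap or door while something overlaps its collision box.
; Overlap begin swaps the mesh to a glow material and activates the referenced actor; overlap end restores the normal material and deactivates it.
; The target is resolved by chained casts to TrapDoor, WaterTrap or BpTubeDoor, printing a failure message if none match.
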(event OnComponentBeginOverlap(CollisionBox)
  (params (OverlappedComponent :type Primitive%20Component%20Object%20Reference) (OtherActor :type Actor%20Object%20Reference) (OtherComp :type Primitive%20Component%20Object%20Reference) (OtherBodyIndex :type Integer) (bFromSweep :type Boolean) (SweepResult :type Hit%20Result%20Structure%20%28by%20ref%29))
  (bind _refactor (Variables|Default|GetRefActor))
  (Rendering|Material|SetMaterial (Variables|Default|GetMesh) 0 (Variables|Default|GetGlowMaterial))
  (bind _astrap_door (Utilities|Casting|CastToTrapDoor _refactor)
    (:then
      (Default|ActivateTrap _astrap_door))
    (:CastFailed
      (bind _aswater_trap (Utilities|Casting|CastToWaterTrap _refactor)
        (:then
          (Default|ActivateTrap _aswater_trap))
        (:CastFailed
          (bind _asbp_tube_door (Utilities|Casting|CastToBpTubeDoor _refactor)
            (:then
              (Default|Activate _asbp_tube_door))
            (:CastFailed
              (Development|PrintString "Failed Cast to BPTubeDoor"))))))))

(event OnComponentEndOverlap(CollisionBox)
  (params (OverlappedComponent :type Primitive%20Component%20Object%20Reference) (OtherActor :type Actor%20Object%20Reference) (OtherComp :type Primitive%20Component%20Object%20Reference) (OtherBodyIndex :type Integer))
  (bind _refactor (Variables|Default|GetRefActor))
  (Rendering|Material|SetMaterial (Variables|Default|GetMesh) 0 (Variables|Default|GetNormalMaterial))
  (bind _astrap_door (Utilities|Casting|CastToTrapDoor _refactor)
    (:then
      (Default|DeactiveTrap _astrap_door))
    (:CastFailed
      (bind _aswater_trap (Utilities|Casting|CastToWaterTrap _refactor)
        (:then
          (Default|DeactivateTrap _aswater_trap))
        (:CastFailed
          (bind _asbp_tube_door (Utilities|Casting|CastToBpTubeDoor _refactor)
            (:then
              (Default|Deactivate _asbp_tube_door))
            (:CastFailed
              (Development|PrintString "Failed Cast to BPTubeDoor"))))))))

(event EventBeginPlay)

(event Collision|EventActorBeginOverlap
  (params (OtherActor :type Actor%20Object%20Reference)))

(event EventTick
  (params (DeltaSeconds :type Float%20%28single-precision%29)))

(fn ConstructionScript)