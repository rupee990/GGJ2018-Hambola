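; SelectionGameMode is the game mode for local multiplayer player selection, run before the game map loads.
; On BeginPlay it shows the PlayerSelection widget, creates three extra local players and has each of the four controllers possess a MenuPawn tagged with its PlayerID.
; PlayerSelection stores selected pawns' IDs in CustomGameInstance and opens Map once more than one is stored.
; RemoveplayerSelection removes an ID from that list.
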(event Custom|PlayerSelection
  (bind _outactors (Actor|GetAllActorsOfClass "/Game/Blueprints/MenuPawn.MenuPawn_C"))
  (bind _ascustom_game_instance (Utilities|Casting|CastToCustomGameInstance (Game|GetGameInstance)))
  (for _array_element _outactors
    (if (Variables|/Game/Blueprints/MenuPawn.MenuPawn_C|GetSelected _array_element)
      (Utilities|Array|AddUnique (Variables|/Game/CustomGameInstance.CustomGameInstance_C|GetPlayersIDs _ascustom_game_instance) (Variables|/Game/Blueprints/MenuPawn.MenuPawn_C|GetPlayerID _array_element))))
  (if (> (Utilities|Array|Length (Variables|/Game/CustomGameInstance.CustomGameInstance_C|GetPlayersIDs _ascustom_game_instance)) 1)
    (Game|OpenLevel(byName) "Map")))

(event Custom|Remove%20player%20Selection
  (params (ID :type Integer))
  (bind _ascustom_game_instance (Utilities|Casting|CastToCustomGameInstance (Game|GetGameInstance)))
  (Utilities|Array|RemoveItem (Variables|/Game/CustomGameInstance.CustomGameInstance_C|GetPlayersIDs _ascustom_game_instance) ID))

(event EventBeginPlay
  (bind _returnvalue (Game|GetPlayerController 0))
  (bind _returnvalue_2 (Math|Transform|MakeTransform "0, 0, 0"))
  (bind _playerarray (Variables|Default|GetPlayerArray))
  (bind _returnvalue_3 (UserInterface|CreateWidget "/Game/Widgets/PlayerSelection.PlayerSelection_C"))
  (UserInterface|Viewport|AddtoViewport _returnvalue_3 0)
  (Utilities|Array|AddUnique _playerarray _returnvalue)
  (bind _returnvalue_4 (Game|SpawnActorfromClass "/Game/Blueprints/MenuPawn.MenuPawn_C" _returnvalue_2 "Undefined" 0 0))
  (Variables|/Game/Blueprints/MenuPawn.MenuPawn_C|SetPlayerID _returnvalue_4 0)
  (Pawn|Possess _returnvalue _returnvalue_4)
  (for _index (range 1 3)
    (bind _returnvalue_5 (Class|GameplayStatics|CreatePlayer _index))
    (Utilities|Array|AddUnique _playerarray _returnvalue_5)
    (bind _returnvalue_6 (Game|SpawnActorfromClass "/Game/Blueprints/MenuPawn.MenuPawn_C" _returnvalue_2 "Undefined" 0 0))
    (Variables|/Game/Blueprints/MenuPawn.MenuPawn_C|SetPlayerID _returnvalue_6 _index)
    (Pawn|Possess _returnvalue_5 _returnvalue_6)))

(event EventTick
  (params (DeltaSeconds :type Float%20%28single-precision%29)))

(fn ConstructionScript)