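; Input pawn Blueprint that passes movement axis input to a Tagged actor in the level.
; On BeginPlay it caches the first Tagged actor found.
; MoveForward adds its axis value to that actor's AdditionalY and MoveRight to AdditionalX, so the offsets accumulate without delta-time scaling.
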(event EventBeginPlay
  (bind _outactors (Actor|GetAllActorsOfClass "/Game/Blueprints/Tagged/Tagged.Tagged_C"))
  (Variables|Default|SetTaggedRef (Utilities|Array|Get(acopy) _outactors)))

(event Collision|EventActorBeginOverlap
  (params (OtherActor :type Actor%20Object%20Reference)))

(event EventTick
  (params (DeltaSeconds :type Float%20%28single-precision%29)))

(event Input|AxisEvents|InputAxisMoveForward
  (params (AxisValue :type Float%20%28single-precision%29))
  (bind _taggedref (Variables|Default|GetTaggedRef))
  (Variables|/Game/Blueprints/Tagged/Tagged.Tagged_C|SetAdditionalY _taggedref (+ AxisValue (Variables|/Game/Blueprints/Tagged/Tagged.Tagged_C|GetAdditionalY _taggedref))))

(event Input|AxisEvents|InputAxisMoveRight
  (params (AxisValue :type Float%20%28single-precision%29))
  (bind _taggedref (Variables|Default|GetTaggedRef))
  (Variables|/Game/Blueprints/Tagged/Tagged.Tagged_C|SetAdditionalX _taggedref (+ AxisValue (Variables|/Game/Blueprints/Tagged/Tagged.Tagged_C|GetAdditionalX _taggedref))))

(fn ConstructionScript)