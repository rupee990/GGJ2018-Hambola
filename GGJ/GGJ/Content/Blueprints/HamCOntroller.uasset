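; HamCOntroller is a controller that forwards global player input to the ThirdPersonGameMode and handles quitting the game.
; The GameStart and TestButton actions cast the current game mode and call PressStart and PressA on it.
; Tick polls the Escape key directly and quits only when the game mode's State is above zero.
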(event EventBeginPlay)

(event EventTick
  (params (DeltaSeconds :type Float%20%28single-precision%29))
  (if (Game|Player|WasInputKeyJustPressed "Escape")
    (bind _asthird_person_game_mode (Utilities|Casting|CastToThirdPersonGameMode (Game|GetGameMode)))
    (if (> (Variables|/Game/Blueprints/GameModes/ThirdPersonGameMode.ThirdPersonGameMode_C|GetState _asthird_person_game_mode) 0)
      (Game|QuitGame 0 "Quit"))))

(event Input|ActionEvents|InputActionGameStart
  (params (Key :type Key%20Structure))
  (:Pressed
    (bind _asthird_person_game_mode (Utilities|Casting|CastToThirdPersonGameMode (Game|GetGameMode)))
    (Default|PressStart _asthird_person_game_mode)))

(event Input|ActionEvents|InputActionTestButton
  (params (Key :type Key%20Structure))
  (:Pressed
    (bind _asthird_person_game_mode (Utilities|Casting|CastToThirdPersonGameMode (Game|GetGameMode)))
    (Default|PressA _asthird_person_game_mode)))

(fn ConstructionScript)