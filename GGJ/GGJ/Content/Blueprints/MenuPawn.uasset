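; MenuPawn is an input pawn for a player selection menu, letting a player join or leave and trigger the game mode's selection step.
; Pressing TestButton toggles Selected, prints it with PlayerID for debugging, then adds or removes that ID through SelectionGameMode.
; Pressing GameStart calls PlayerSelection on the same game mode.
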(event EventBeginPlay)

(event Collision|EventActorBeginOverlap
  (params (OtherActor :type Actor%20Object%20Reference)))

(event EventTick
  (params (DeltaSeconds :type Float%20%28single-precision%29)))

(event Input|ActionEvents|InputActionTestButton
  (params (Key :type Key%20Structure))
  (:Pressed
    (bind _output_get (Variables|Default|SetSelected (not (Variables|Default|GetSelected))))
    (if _output_get
      (Development|PrintString (Utilities|String|Append (Utilities|String|ToString(Boolean) _output_get) (Utilities|String|ToString(Integer) (Variables|Default|GetPlayerID))))
      (bind _asselection_game_mode (Utilities|Casting|CastToSelectionGameMode (Game|GetGameMode)))
      (Default|AddPlayer _asselection_game_mode (Variables|Default|GetPlayerID))
      (else
        (Development|PrintString (Utilities|String|Append (Utilities|String|ToString(Boolean) _output_get) (Utilities|String|ToString(Integer) (Variables|Default|GetPlayerID))))
        (bind _asselection_game_mode_2 (Utilities|Casting|CastToSelectionGameMode (Game|GetGameMode)))
        (Default|RemovePlayer _asselection_game_mode_2 (Variables|Default|GetPlayerID))))))

(event Input|ActionEvents|InputActionGameStart
  (params (Key :type Key%20Structure))
  (:Pressed
    (bind _asselection_game_mode (Utilities|Casting|CastToSelectionGameMode (Game|GetGameMode)))
    (Default|PlayerSelection _asselection_game_mode)))

(fn ConstructionScript)