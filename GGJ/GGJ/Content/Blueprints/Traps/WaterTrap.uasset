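; Water trap that spreads a puddle when activated and flags Tagged or untagged actors overlapping it as InWater.
; Activation reveals the puddle, enables its collision and plays audio; deactivation waits briefly, then disables collision.
; Tick steps the puddle's scale up or down from the GrowPuddle flag, hiding it once shrunk.
; Overlap events set and clear InWater only while PuddleActive, which deactivation clears before disabling collision.
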(event OnComponentBeginOverlap(PuddleCol)
  (params (OverlappedComponent :type Primitive%20Component%20Object%20Reference) (OtherActor :type Actor%20Object%20Reference) (OtherComp :type Primitive%20Component%20Object%20Reference) (OtherBodyIndex :type Integer) (bFromSweep :type Boolean) (SweepResult :type Hit%20Result%20Structure%20%28by%20ref%29))
  (if (Variables|Default|GetPuddleActive)
    (bind _astagged (Utilities|Casting|CastToTagged OtherActor)
      (:then
        (Variables|/Game/Blueprints/Tagged/Tagged.Tagged_C|SetInWater _astagged true))
      (:CastFailed
        (bind _asuntagged (Utilities|Casting|CastTountagged OtherActor))
        (Variables|/Game/Blueprints/untagged/untagged.untagged_C|SetInWater _asuntagged true)))))

(event OnComponentEndOverlap(PuddleCol)
  (params (OverlappedComponent :type Primitive%20Component%20Object%20Reference) (OtherActor :type Actor%20Object%20Reference) (OtherComp :type Primitive%20Component%20Object%20Reference) (OtherBodyIndex :type Integer))
  (if (Variables|Default|GetPuddleActive)
    (bind _astagged (Utilities|Casting|CastToTagged OtherActor)
      (:then
        (Variables|/Game/Blueprints/Tagged/Tagged.Tagged_C|SetInWater _astagged false))
      (:CastFailed
        (bind _asuntagged (Utilities|Casting|CastTountagged OtherActor))
        (Variables|/Game/Blueprints/untagged/untagged.untagged_C|SetInWater _asuntagged false)))))

(event Custom|ActivateTrap
  (bind _puddlecol (Variables|Default|GetPuddleCol))
  (Utilities|FlowControl|Delay 0.0)
  (Rendering|SetVisibility (Variables|Default|GetPuddle) true false)
  (Collision|SetCollisionEnabled _puddlecol "QueryAndPhysics")
  (Rendering|Material|SetMaterial _puddlecol 0 "/Game/Materials/WaterButtonPressed.WaterButtonPressed")
  (Variables|Default|SetPuddleActive true)
  (Variables|Default|SetGrowPuddle true)
  (Audio|Components|Audio|Play (Variables|Default|GetAudio) 0.0))

(event Custom|DeactivateTrap
  (Utilities|FlowControl|Delay 2.5)
  (Variables|Default|SetPuddleActive false)
  (Variables|Default|SetGrowPuddle false)
  (Collision|SetCollisionEnabled (Variables|Default|GetPuddleCol) "NoCollision"))

(event EventBeginPlay
  (Rendering|SetVisibility (Variables|Default|GetPuddle) false false)
  (Collision|SetCollisionEnabled (Variables|Default|GetPuddleCol) "NoCollision"))

(event EventTick
  (params (DeltaSeconds :type Float%20%28single-precision%29))
  (bind _puddle (Variables|Default|GetPuddle))
  (bind _puddle_2 (Variables|Default|GetPuddle))
  (bind _puddle_3 (Variables|Default|GetPuddle))
  (bind _puddle_4 (Variables|Default|GetPuddle))
  (bind _returnvalue (Transformation|GetWorldScale _puddle_3))
  (bind _returnvalue_2 (Transformation|GetWorldScale _puddle_4))
  (bind _returnvalue_3 (Transformation|GetWorldScale _puddle))
  (bind _returnvalue_4 (Transformation|GetWorldScale _puddle_2))
  (bind (_x _y) (Math|Vector|BreakVector _returnvalue_2))
  (bind (_x_2 _y_2) (Math|Vector|BreakVector _returnvalue))
  (bind (_x_3 _y_3) (Math|Vector|BreakVector _returnvalue_3))
  (bind (_x_4 _y_4) (Math|Vector|BreakVector _returnvalue_4))
  (if (Variables|Default|GetGrowPuddle)
    (if (and (< _x_3 2.5) (< _y_3 2.5))
      (Transformation|SetWorldScale3D (Variables|Default|GetPuddle) (Math|Vector|MakeVector (+ _x_4 0.1) (+ _y_4 0.1) 0.0)))
    (elif (and (>= _x 0.5) (>= _y 0.5))
      (Transformation|SetWorldScale3D (Variables|Default|GetPuddle) (Math|Vector|MakeVector (- _x_2 0.1) (- _y_2 0.1) 0.0))
      (else
        (Rendering|SetVisibility (Variables|Default|GetPuddle) false false)))))

(fn ConstructionScript)