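; Tube door trap that swings shut when activated and opens when deactivated, toggling whether the linked TubeEnd2 can be passed.
; Tick steps the mesh's world roll between shut and a fixed open angle at separate open and close rates, playing audio once on fully closing.
; OpenToAngle is set but never read here, and the TubeEnd1 pass toggles are disconnected.
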(event Custom|Activate
  (Variables|/Game/Blueprints/BpPipe.BpPipe_C|SetCanPass (Variables|Default|GetTubeEnd2) false)
  (Variables|Default|SetOpen false)
  (Variables|Default|SetOpenToAngle 0.0))

(event Custom|Deactivate
  (Variables|/Game/Blueprints/BpPipe.BpPipe_C|SetCanPass (Variables|Default|GetTubeEnd2) true)
  (Variables|Default|SetOpen true)
  (Variables|Default|SetOpenToAngle 0.0))

(event EventTick
  (params (DeltaSeconds :type Float%20%28single-precision%29))
  (bind _staticmeshcomponent (Variables|Debug|GetStaticMeshComponent))
  (bind _staticmeshcomponent_2 (Variables|Debug|GetStaticMeshComponent))
  (bind _returnvalue (Transformation|GetWorldRotation _staticmeshcomponent))
  (bind _returnvalue_2 (Transformation|GetWorldRotation _staticmeshcomponent_2))
  (bind (_roll _pitch _yaw) (Math|Rotator|BreakRotator _returnvalue))
  (bind (_roll_2 _pitch_2 _yaw_2) (Math|Rotator|BreakRotator _returnvalue_2))
  (if (Variables|Default|GetOpen)
    (if (< (Variables|Default|GetOpenAngle) 1.4e+02)
      (bind _output_get (Variables|Default|SetOpenAngle (+ (Variables|Default|GetOpenAngle) (Variables|Default|GetOpenRate))))
      (Transformation|SetWorldRotation (Variables|Debug|GetStaticMeshComponent) (Math|Rotator|MakeRotator _output_get _pitch _yaw) false false))
    (elif (> (Variables|Default|GetOpenAngle) 0.0)
      (Variables|Default|SetClosed false)
      (bind _output_get_2 (Variables|Default|SetOpenAngle (- (Variables|Default|GetOpenAngle) (Variables|Default|GetCloseRate))))
      (Transformation|SetWorldRotation (Variables|Debug|GetStaticMeshComponent) (Math|Rotator|MakeRotator _output_get_2 _pitch_2 _yaw_2) false false)
      (elif (not (Variables|Default|GetClosed))
        (Variables|Default|SetClosed true)
        (Audio|Components|Audio|Play (Variables|Default|GetAudio) 0.0)))))

(fn ConstructionScript)