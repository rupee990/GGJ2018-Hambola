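; Trapdoor trap that opens by vanishing and losing collision, then closes by restoring both.
; ActivateTrap waits briefly, hides TrapdoorMesh, disables its collision and plays the Audio component.
; DeactiveTrap waits the same short delay, then shows the mesh and re-enables query and physics collision, without sound.
; Neither event is called within this Blueprint, and the construction script is empty.
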(event Custom|ActivateTrap
  (bind _trapdoormesh (Variables|Default|GetTrapdoorMesh))
  (Utilities|FlowControl|Delay 0.2)
  (Rendering|SetVisibility _trapdoormesh false false)
  (Collision|SetCollisionEnabled _trapdoormesh "NoCollision")
  (Audio|Components|Audio|Play (Variables|Default|GetAudio) 0.0))

(event Custom|DeactiveTrap
  (bind _trapdoormesh (Variables|Default|GetTrapdoorMesh))
  (Utilities|FlowControl|Delay 0.2)
  (Rendering|SetVisibility _trapdoormesh true false)
  (Collision|SetCollisionEnabled _trapdoormesh "QueryAndPhysics"))

(fn ConstructionScript)